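; Key actor that is shown with collision enabled only when no BP_Target_2 actors remain in the level.
; Tick checks this every frame via the index returned by an array Add, then sets the flag true regardless and fires a one-time appear effect and sound, unconditionally.
; BeginPlay caches the player character, but the overlap event is empty and the pickup logic that grants HasKey is disconnected.
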(event `self.ReceiveTick`
  (params (DeltaSeconds :type "Float (single-precision)"))
  (bind _returnvalue (`SceneComponent.K2_GetComponentLocation` (`self.SM_Key_Temp`)))
  (bind _outactors (`GameplayStatics.GetAllActorsOfClass` "/Game/MyContent/Blueprints/BP_Target_2.BP_Target_2_C"))
  (bind _returnvalue_2 (`KismetArrayLibrary.Array_Add` _outactors))
  (bind _output_get (set `self.All_Targets_Are_Destroyed` (<= _returnvalue_2 0)))
  (`SceneComponent.SetVisibility` (`self.SM_Key_Temp`) _output_get false)
  (`self.SetActorEnableCollision` _output_get)
  (set `self.All_Targets_Are_Destroyed` true)
  (`/Engine/EditorBlueprintResources/StandardMacros.DoOnce` false
    (:`Completed`
      (`NiagaraFunctionLibrary.SpawnSystemAtLocation` "/Game/MyContent/FX/PE_Key_Hit.PE_Key_Hit" _returnvalue)
      (`GameplayStatics.SpawnSoundAtLocation` "/Game/MyContent/Audio/MP3_Key_Appear.MP3_Key_Appear" _returnvalue (struct) 1.0 1.0 0.0 null null))))

(event `self.ReceiveBeginPlay`
  (bind _asbp_first_person_character (cast `/Game/StarterContent/FirstPerson/Blueprints/BP_FirstPersonCharacter` (`GameplayStatics.GetPlayerCharacter` 0)))
  (set `self.BP First Person Character` _asbp_first_person_character))

(event `self.Collision.OnComponentBeginOverlap`
  (params (OverlappedComponent :type "PrimitiveComponent Object Reference") (OtherActor :type "Actor Object Reference") (OtherComp :type "PrimitiveComponent Object Reference") (OtherBodyIndex :type Integer) (bFromSweep :type Boolean) (SweepResult :type "HitResult Structure (by ref)")))

(fn `UserConstructionScript`)