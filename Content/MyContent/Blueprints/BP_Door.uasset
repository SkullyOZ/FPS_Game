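; BP_Door is a door Blueprint whose indicator light shows whether the player holds a key.
; BeginPlay caches the first-person character, applies a dynamic material instance of MI_Door_Light to the light mesh and sets it green.
; When that character enters the collision volume, the light's intensity rises and its colour becomes green with HasKey, red without.
; End overlap does nothing, and the file contains no door-opening logic.
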(event `self.ReceiveBeginPlay`
  (bind _asbp_first_person_character (cast `/Game/StarterContent/FirstPerson/Blueprints/BP_FirstPersonCharacter` (`GameplayStatics.GetPlayerCharacter` 0)))
  (set `self.BP First Person Character` _asbp_first_person_character)
  (bind _returnvalue (`KismetMaterialLibrary.CreateDynamicMaterialInstance` "/Game/MyContent/Materials/MI_Door_Light.MI_Door_Light"))
  (set `self.Dynamic Material` _returnvalue)
  (`PrimitiveComponent.SetMaterial` (`self.SM_Light`) 0 (`self.Dynamic Material`))
  (`MaterialInstanceDynamic.SetVectorParameterValue` (`self.Dynamic Material`) "Colour" (struct :`R` 0.036118 :`G` 1.0 :`B` 0.010886 :`A` 1.0) :!label _label))

(event `self.Collision.OnComponentBeginOverlap`
  (params (OverlappedComponent :type "PrimitiveComponent Object Reference") (OtherActor :type "Actor Object Reference") (OtherComp :type "PrimitiveComponent Object Reference") (OtherBodyIndex :type Integer) (bFromSweep :type Boolean) (SweepResult :type "HitResult Structure (by ref)"))
  (if (== OtherActor (`self.BP First Person Character`))
    (`MaterialInstanceDynamic.SetScalarParameterValue` (`self.Dynamic Material`) "Intensity" 100.0)
    (if (`/Game/StarterContent/FirstPerson/Blueprints/BP_FirstPersonCharacter.HasKey` (`self.BP First Person Character`))
      (goto _label)
      (else
        (`MaterialInstanceDynamic.SetVectorParameterValue` (`self.Dynamic Material`) "Colour" (struct :`R` 1.0 :`G` 0.00094 :`A` 1.0))))))

(event `self.Collision.OnComponentEndOverlap`
  (params (OverlappedComponent :type "PrimitiveComponent Object Reference") (OtherActor :type "Actor Object Reference") (OtherComp :type "PrimitiveComponent Object Reference") (OtherBodyIndex :type Integer)))

(fn `UserConstructionScript`)